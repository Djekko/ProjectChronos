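; Fire hazard actor that marks the first-person player as inside a damage area while they overlap it.
; On BeginPlay it caches the FirstPersonCharacter, then DamageArea overlaps with that player's capsule set or clear IsInDamageArea.
; Entering also writes the start time and fire location to the character, and no damage is applied in this Blueprint.
; A world camera shake node is present but never runs.
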(event OnComponentBeginOverlap(DamageArea)
  (params (OverlappedComponent :type Primitive%20Component%20Object%20Reference) (OtherActor :type Actor%20Object%20Reference) (OtherComp :type Primitive%20Component%20Object%20Reference) (OtherBodyIndex :type Integer) (bFromSweep :type Boolean) (SweepResult :type Hit%20Result%20Structure%20%28by%20ref%29))
  (if (== OtherComp (Variables|/Script/Engine.Character|GetCapsuleComponent (Variables|Default|GetPlayer)))
    (Variables|/Script/ProjectChronosTests.ProjectChronosTestsCharacter|SetdamageStartTime (Variables|Default|GetPlayer) (Utilities|Time|GetRealTimeSeconds))
    (Variables|/Script/ProjectChronosTests.ProjectChronosTestsCharacter|SetDamageLocation (Variables|Default|GetPlayer) (Transformation|GetWorldLocation (Variables|Default|GetDefaultSceneRoot)))
    (Variables|/Script/ProjectChronosTests.ProjectChronosTestsCharacter|SetbIsInDamageArea (Variables|Default|GetPlayer) true)))

(event OnComponentEndOverlap(DamageArea)
  (params (OverlappedComponent :type Primitive%20Component%20Object%20Reference) (OtherActor :type Actor%20Object%20Reference) (OtherComp :type Primitive%20Component%20Object%20Reference) (OtherBodyIndex :type Integer))
  (if (== OtherComp (Variables|/Script/Engine.Character|GetCapsuleComponent (Variables|Default|GetPlayer)))
    (Variables|/Script/ProjectChronosTests.ProjectChronosTestsCharacter|SetbIsInDamageArea (Variables|Default|GetPlayer) false)))

(event EventBeginPlay
  (Variables|Default|SetPlayer (.AsFirst%20Person%20Character (Utilities|Casting|CastToFirstPersonCharacter (Game|GetPlayerCharacter 0)))))

(fn ConstructionScript)