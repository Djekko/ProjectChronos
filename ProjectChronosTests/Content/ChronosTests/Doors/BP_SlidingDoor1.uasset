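; BP_SlidingDoor1 is an automatic sliding door with outer and inner panel pairs that opens when something overlaps its trigger box.
; On BeginPlay a locked door destroys the trigger, while an unlocked one hides its inner panels.
; Overlap plays a timeline that moves each pair in mirrored directions.
; When an overlap ends, the timeline reverses only if no FirstPersonCharacter or AI_ShooterCharacter remains inside.
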(event OnComponentBeginOverlap(Box)
  (params (OverlappedComponent :type Primitive%20Component%20Object%20Reference) (OtherActor :type Actor%20Object%20Reference) (OtherComp :type Primitive%20Component%20Object%20Reference) (OtherBodyIndex :type Integer) (bFromSweep :type Boolean) (SweepResult :type Hit%20Result%20Structure%20%28by%20ref%29))
  (bind (_direction _innerdoor _outerdoor) (Timeline|DoorOpenClose Play)
    (:Update
      (Transformation|SetRelativeLocation (Variables|Default|GetDoorOuterTop) _outerdoor false false)
      (Transformation|SetRelativeLocation (Variables|Default|GetDoorInnerBottom) _innerdoor false false)
      (Transformation|SetRelativeLocation (Variables|Default|GetDoorOuterBottom) (* _outerdoor -1.0) false false)
      (Transformation|SetRelativeLocation (Variables|Default|GetDoorInnerTop) (* _innerdoor -1.0) false false))))

(event OnComponentEndOverlap(Box)
  (params (OverlappedComponent :type Primitive%20Component%20Object%20Reference) (OtherActor :type Actor%20Object%20Reference) (OtherComp :type Primitive%20Component%20Object%20Reference) (OtherBodyIndex :type Integer))
  (bind _box (Variables|Default|GetBox))
  (if (== (+ (Utilities|Array|Length (Collision|GetOverlappingActors _box "/Game/FirstPersonCPP/Blueprints/FirstPersonCharacter.FirstPersonCharacter_C" :!class /Script/Engine.PrimitiveComponent)) (Utilities|Array|Length (Collision|GetOverlappingActors _box "/Game/ThirdPersonBP/Blueprints/AI_ShooterCharacter.AI_ShooterCharacter_C" :!class /Script/Engine.PrimitiveComponent))) 0)
    (bind (_direction _innerdoor _outerdoor) (Timeline|DoorOpenClose Reverse)
      (:Update
        (Transformation|SetRelativeLocation (Variables|Default|GetDoorOuterTop) _outerdoor false false)
        (Transformation|SetRelativeLocation (Variables|Default|GetDoorInnerBottom) _innerdoor false false)
        (Transformation|SetRelativeLocation (Variables|Default|GetDoorOuterBottom) (* _outerdoor -1.0) false false)
        (Transformation|SetRelativeLocation (Variables|Default|GetDoorInnerTop) (* _innerdoor -1.0) false false)))))

(event EventBeginPlay
  (if (Variables|Default|GetisDoorLocked)
    (Components|DestroyComponent (Variables|Default|GetBox))
    (else
      (Rendering|SetVisibility (Variables|Default|GetDoorInnerBottom) false false)
      (Rendering|SetVisibility (Variables|Default|GetDoorInnerTop) false false))))

(fn ConstructionScript)