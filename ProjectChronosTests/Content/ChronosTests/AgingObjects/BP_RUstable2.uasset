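; BP_RUstable2 makes its owning actor an "AgeableObject" that the player can age into rust, then dissolve and destroy.
; On BeginPlay it gives the first static mesh a dynamic M_DynamicRust instance.
; While the player's line trace hits it, Tick raises "Blend" during interaction, using a time offset to resume after pauses.
; Once rusted, it enables physics, drops the tag and drives "Dissolve" down while still traced, without needing interaction.
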(event EventBeginPlay
  (Utilities|Array|Add (Variables|/Script/Engine.Actor|GetTags (Components|GetOwner)) "AgeableObject")
  ;[1 1 1] get player ref
  (Variables|Default|SetPlayer (.AsFirst%20Person%20Character (Utilities|Casting|CastToFirstPersonCharacter (Game|GetPlayerCharacter 0))))
  ;[1 1 1] get owner ref
  (bind _output_get (Variables|Default|SetOwner (Utilities|Array|Get(acopy) (Actor|GetComponentsByClass (Components|GetOwner self) "/Script/Engine.StaticMeshComponent"))))
  (Variables|/Script/Engine.PrimitiveComponent|SetbGenerateOverlapEvents _output_get true)
  ;[1 1 1] set to rustable mat
  (Rendering|Material|SetMaterial (Variables|Default|GetOwner) 0 "/Game/ChronosTests/AgingObjects/M_DynamicRust.M_DynamicRust")
  ;[1 1 1] Create a Unique Mat Instance
  (bind _returnvalue (Rendering|Material|CreateDynamicMaterialInstance (Variables|Default|GetOwner) 0 (Rendering|Material|GetMaterial (Variables|Default|GetOwner) 0) :!class /Script/Engine.PrimitiveComponent))
  (Variables|Default|SetMatInstance _returnvalue))

(event EventTick
  (params (DeltaSeconds :type Float%20%28single-precision%29))
  (bind _increse_alpha_value (Utilities|IncreseAlphaValue))
  (bind _decrese_alpha_value (Utilities|DecreseAlphaValue))
  (if (== (Components|GetOwner (Variables|Default|GetOwner)) (Variables|/Game/FirstPersonCPP/Blueprints/FirstPersonCharacter.FirstPersonCharacter_C|GetLineTraceActorHit (Variables|Default|GetPlayer)))
    ;[1 1 1] If the Actor is no longer visable
    (if (Variables|Default|GetHasDissolved)
      (Actor|DestroyActor (Components|GetOwner (Variables|Default|GetOwner)))
      (else
        ;[1 1 1] Is the object already rusted
        (if (Variables|Default|GetHasRusted)
          ;[1 1 1] Change the Mat Instance Alpha For Disolving Over 3 seconds
          (Variables|Default|SetIsDissolving true)
          (if (<= _decrese_alpha_value 0.0)
            (Variables|Default|SetPerameterValue 0.0)
            (Variables|Default|SetHasDissolved true)
            (else
              (Variables|Default|SetPerameterValue _decrese_alpha_value)))
          (Rendering|Material|SetScalarParameterValue (Variables|Default|GetMatInstance) "Dissolve" (Variables|Default|GetPerameterValue) :!class /Script/Engine.MaterialInstanceDynamic)
          (else
            ;[1 1 1] if the owner was not hit do nothing
            (if (Variables|/Game/FirstPersonCPP/Blueprints/FirstPersonCharacter.FirstPersonCharacter_C|GetbAgeableInteract (Variables|Default|GetPlayer))
              (if (Variables|Default|GetNeedToSetNewStartTimeOffset)
                (Variables|Default|SetTimeOffset (Variables|Default|GetTimePassedOnObject))
                (Variables|Default|SetNeedToSetNewStartTimeOffset false))
              (Variables|Default|SetStartTime (Variables|/Game/FirstPersonCPP/Blueprints/FirstPersonCharacter.FirstPersonCharacter_C|GetInteractionStartTime (Variables|Default|GetPlayer)))
              ;[1 1 1] Change the Mat Instance Alpha For Rusting Over 3 Seconds
              (Variables|Default|SetIsRusting true)
              (if (>= _increse_alpha_value 1.0)
                (Variables|Default|SetPerameterValue 1.0)
                (Variables|Default|SetHasRusted true)
                (Physics|SetSimulatePhysics (Variables|Default|GetOwner) true)
                (Variables|Default|SetStartTime (Utilities|Time|GetRealTimeSeconds))
                (Utilities|Array|RemoveItem (Variables|/Script/Engine.Actor|GetTags (Components|GetOwner)) "AgeableObject")
                (else
                  (Variables|Default|SetPerameterValue _increse_alpha_value)
                  (Variables|Default|SetTimePassedOnObject (- (+ (Utilities|Time|GetRealTimeSeconds) (Variables|Default|GetTimeOffset)) (Variables|Default|GetStartTime)))))
              (Rendering|Material|SetScalarParameterValue (Variables|Default|GetMatInstance) "Blend" (Variables|Default|GetPerameterValue) :!class /Script/Engine.MaterialInstanceDynamic)
              (else
                (Variables|Default|SetNeedToSetNewStartTimeOffset true)))))))))