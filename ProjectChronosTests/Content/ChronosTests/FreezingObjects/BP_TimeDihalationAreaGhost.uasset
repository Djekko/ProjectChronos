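; Ghost actor for the time dilation area, meant to sit in front of the first-person player.
; BeginPlay caches the FirstPersonCharacter, and every Tick moves the root component to the result of GetGhostPos without sweeping.
; GetGhostPos holds a camera-forward projection scaled by the player's DilationAreaDistanceBP, but that calculation appears unconnected to any output.
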(event EventTick
  (params (DeltaSeconds :type Float%20%28single-precision%29))
  ;[0.07075 1 0] Comment
  ;;[1 1 1] GeetTheGhostInFrontOfThePlayer
  (Transformation|SetWorldLocation (Variables|Default|GetDefaultSceneRoot self) (Utilities|GetGhostPos) false false))

(event EventBeginPlay
  ;[0.07075 1 0] Comment
  ;;[1 1 1] GetPlayerRef
  (Variables|Default|SetPlayer (.AsFirst%20Person%20Character (Utilities|Casting|CastToFirstPersonCharacter (Game|GetPlayerCharacter 0)))))

(fn ConstructionScript)