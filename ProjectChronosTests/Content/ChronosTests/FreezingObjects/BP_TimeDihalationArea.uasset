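; Time dilation volume that scales via a timeline and slows non-exempt actors inside it through CustomTimeDilation, applied on Tick.
; Physics slowing is faked by scaling velocities and toggling gravity on overlap.
; A player inside inverts the effect, raising global dilation while lowering their own and the volume's.
; Changes in the player's rewind state reverse the timeline, and volume destruction can be logged on the player for rewinding.
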(event OnComponentBeginOverlap(Cylinder)
  (params (OverlappedComponent :type Primitive%20Component%20Object%20Reference) (OtherActor :type Actor%20Object%20Reference) (OtherComp :type Primitive%20Component%20Object%20Reference) (OtherBodyIndex :type Integer) (bFromSweep :type Boolean) (SweepResult :type Hit%20Result%20Structure%20%28by%20ref%29))
  ;[0.03957 1 0] Comment
  (Variables|Default|SetOverlappingActor OtherActor)
  (Variables|Default|SetBeginOverLappingComp OtherComp)
  ;;[1 1 1] Is the overlapping actor the player
  (if (== "/Game/FirstPersonCPP/Blueprints/FirstPersonCharacter.FirstPersonCharacter_C" (Utilities|GetClass (Variables|Default|GetOverlappingActor)))
    ;;[1 1 1] any objects that enter keep there gravity
    (CallFunction|FakeSlowDilation (Variables|Default|GetBeginOverLappingComp) true)
    ;;[1 1 1] Set time dilation for player and world
    (Utilities|Time|SetGlobalTimeDilation 2e+01)
    (Variables|Default|SetCustomTimeDilation (Variables|Default|GetOverlappingActor) 0.05)
    ;;[1 1 1] Set custom dilation for the area to not speed up the delay
    (Variables|Default|SetCustomTimeDilation self 0.05)
    ;;[1 1 1] Any objects already in area enable gravity
    (for _array_element (Class|PrimitiveComponent|GetOverlappingComponents (Variables|Default|GetCylinder))
      (Physics|SetEnableGravity _array_element true))
    (else
      ;;[1 1 1] fake slowing time for static objects
      (CallFunction|FakeSlowDilation (Variables|Default|GetBeginOverLappingComp) false))))

(event OnComponentEndOverlap(Cylinder)
  (params (OverlappedComponent :type Primitive%20Component%20Object%20Reference) (OtherActor :type Actor%20Object%20Reference) (OtherComp :type Primitive%20Component%20Object%20Reference) (OtherBodyIndex :type Integer))
  ;[0.03957 1 0] Comment
  (Variables|Default|SetEndOverlappingActor OtherActor)
  ;;[1 1 1] FakeSettingSlowing obejcts back to normal speed
  (CallFunction|FakeNormalDilation OtherComp)
  ;;[1 1 1] Set custom Dilation
  (Variables|/Script/Engine.Actor|SetCustomTimeDilation (Variables|Default|GetEndOverlappingActor) 1.0)
  ;;[1 1 1] Is the overlapping actor the player
  (if (== "/Game/FirstPersonCPP/Blueprints/FirstPersonCharacter.FirstPersonCharacter_C" (Utilities|GetClass (Variables|Default|GetEndOverlappingActor)))
    (Utilities|Time|SetGlobalTimeDilation 1.0)
    (Variables|Default|SetCustomTimeDilation (Variables|Default|GetEndOverlappingActor) 1.0)
    ;;[1 1 1] Set the area dilation back to normal
    (Variables|Default|SetCustomTimeDilation self 1.0)
    ;;[1 1 1] Any objects are in the area when the player leaves disable gravity
    (for _array_element (Class|PrimitiveComponent|GetOverlappingComponents (Variables|Default|GetCylinder))
      (Physics|SetEnableGravity _array_element false))))

(event Custom|Reverse%20FreezeTimeVolume
  ;[0 1 0.1907] Comment
  ;;[1 1 1] Set scale to 0 and expand
  (bind _singularityscale (Timeline|VolumeExpand Reverse)
    (:Update
      (Transformation|SetActorScale3D self _singularityscale))
    (:Finished
      ;;;[0 0.2118 1] TimeRewindStuff
      (if (Variables|Default|GetReversingFreezeVolumeBP)
        (Actor|DestroyActor self :!label _label)
        (elif (Variables|Default|GetSpawnedReversingBP)
          (goto _label)
          (else
            (Utilities|Array|Add (Variables|/Game/FirstPersonCPP/Blueprints/FirstPersonCharacter.FirstPersonCharacter_C|GetActorDestroyedBP (Variables|Default|GetPlayer)) "BP_TimeDihalationArea_C")
            (Utilities|Array|Add (Variables|/Game/FirstPersonCPP/Blueprints/FirstPersonCharacter.FirstPersonCharacter_C|GetDestroyed%20timeBP (Variables|Default|GetPlayer)) (Utilities|Time|GetRealTimeSeconds))
            (Utilities|Array|Add (Variables|/Game/FirstPersonCPP/Blueprints/FirstPersonCharacter.FirstPersonCharacter_C|GetDestroyedTransformBP (Variables|Default|GetPlayer)) (Transformation|GetActorTransform self))
            (Actor|DestroyActor self)))))))

(event EventTick
  (params (DeltaSeconds :type Float%20%28single-precision%29))
  ;[0.03957 1 0] Comment
  ;;[0.03732 0.05826 0.415] RewindStuff
  (if (Variables|Default|GetSpawnedReversingBP)
    (if (Variables|/Script/ProjectChronosTests.ProjectChronosTestsCharacter|GetbReverseButtonPressed (Variables|Default|GetPlayer))
      _
      (else
        (if (Variables|Default|GetReversingFreezeVolumeBP) :!label _label
          _
          (else
            (Variables|Default|SetReversingFreezeVolumeBP true)
            (CallFunction|ReverseFreezeTimeVolume)))))
    (elif (Variables|/Script/ProjectChronosTests.ProjectChronosTestsCharacter|GetbReverseButtonPressed (Variables|Default|GetPlayer))
      (goto _label)
      (else
        _)))
  ;;[1 1 1] for Each Overlapping Actor in the area
  (for _array_element (Collision|GetOverlappingActors (Variables|Default|GetCylinder) 0 :!class /Script/Engine.PrimitiveComponent)
    (Variables|Default|SetArrayElement _array_element)
    ;;[1 1 1] Is the element Itself
    (if (not (== (Variables|Default|GetArrayElement) self))
      ;;[1 1 1] Is the Actor Exempt From Effects
      (if (not (Utilities|IsTimeExempt (Variables|Default|GetArrayElement)))
        ;;[1 1 1] Set CustomTimeDilation
        (Variables|/Script/Engine.Actor|SetCustomTimeDilation (Variables|Default|GetArrayElement) (Variables|Default|GetTimeDilationBP))))))

(event EventBeginPlay
  ;[0 1 0.1907] Comment
  ;;[1 1 1] get Player Ref
  (Variables|Default|SetPlayer (.AsFirst%20Person%20Character (Utilities|Casting|CastToFirstPersonCharacter (Game|GetPlayerCharacter 0))))
  ;;[0 0.206 1] TimeRewindStuff
  (if (Variables|/Script/ProjectChronosTests.ProjectChronosTestsCharacter|GetbReverseButtonPressed (Variables|Default|GetPlayer))
    (Variables|Default|SetSpawnedReversingBP true)
    ;;[1 1 1] Set scale to 0 and expand
    (bind _singularityscale (Timeline|VolumeExpand PlayFromStart)
      (:Update
        (Transformation|SetActorScale3D self _singularityscale))
      (:Finished
        ;;;[0 0.2118 1] TimeRewindStuff
        (if (Variables|Default|GetReversingFreezeVolumeBP)
          (Actor|DestroyActor self :!label _label)
          (elif (Variables|Default|GetSpawnedReversingBP)
            (goto _label)
            (else
              (Utilities|Array|Add (Variables|/Game/FirstPersonCPP/Blueprints/FirstPersonCharacter.FirstPersonCharacter_C|GetActorDestroyedBP (Variables|Default|GetPlayer)) "BP_TimeDihalationArea_C")
              (Utilities|Array|Add (Variables|/Game/FirstPersonCPP/Blueprints/FirstPersonCharacter.FirstPersonCharacter_C|GetDestroyed%20timeBP (Variables|Default|GetPlayer)) (Utilities|Time|GetRealTimeSeconds))
              (Utilities|Array|Add (Variables|/Game/FirstPersonCPP/Blueprints/FirstPersonCharacter.FirstPersonCharacter_C|GetDestroyedTransformBP (Variables|Default|GetPlayer)) (Transformation|GetActorTransform self))
              (Actor|DestroyActor self))))))
    (else
      (Variables|Default|SetSpawnedReversingBP false)
      (Timeline|VolumeExpand PlayFromStart))))

(fn ConstructionScript)

(fn FakeSlowDilation
  (params (ComponentToEffect :type Primitive%20Component%20Object%20Reference) (EnableGravity :type Boolean))
  (Physics|SetEnableGravity ComponentToEffect EnableGravity)
  (bind _returnvalue (Physics|GetPhysicsLinearVelocity ComponentToEffect "None"))
  (Physics|SetPhysicsLinearVelocity ComponentToEffect (/ _returnvalue 2e+01) false "None")
  (bind _returnvalue_2 (Class|PrimitiveComponent|GetPhysicsAngularVelocity ComponentToEffect "None"))
  (Class|PrimitiveComponent|SetPhysicsAngularVelocity ComponentToEffect (/ _returnvalue_2 2e+01) false "None"))

(fn FakeNormalDilation
  (params (ComponentToEffect :type Primitive%20Component%20Object%20Reference))
  (Physics|SetEnableGravity ComponentToEffect true)
  (bind _returnvalue (Physics|GetPhysicsLinearVelocity ComponentToEffect "None"))
  (Physics|SetPhysicsLinearVelocity ComponentToEffect (* _returnvalue 5.0) false "None")
  (bind _returnvalue_2 (Class|PrimitiveComponent|GetPhysicsAngularVelocity ComponentToEffect "None"))
  (Class|PrimitiveComponent|SetPhysicsAngularVelocity ComponentToEffect (* _returnvalue_2 5.0) false "None"))