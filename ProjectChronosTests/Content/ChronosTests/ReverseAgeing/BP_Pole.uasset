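; Reverse-ageing pole that the player rebuilds from scattered pieces by holding interact on it, draining energy.
; BeginPlay saves the assembled transforms, then scatters the parts to target-actor locations with random rotations.
; Tick lerps parts back over TravelTime, driving a material "Blend" parameter through dynamic instances created each update.
; Interrupting or exhausting energy re-enables physics on the parts; completion locks the pole and clears its interaction tag and prompt.
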(event Custom|PressButton
  (bind _player (Variables|Default|GetPlayer))
  (bind _player_2 (Variables|Default|GetPlayer))
  (if (== (Variables|/Game/FirstPersonCPP/Blueprints/FirstPersonCharacter.FirstPersonCharacter_C|GetLineTraceActorHitBP (Variables|Default|GetPlayer)) self)
    (if (Variables|/Game/FirstPersonCPP/Blueprints/FirstPersonCharacter.FirstPersonCharacter_C|GetbInterationPressedBP (Variables|Default|GetPlayer))
      ;[1 1 1] has it already been built
      (if (not (Variables|Default|GetIsObjectBuilt))
        ;[1 1 1] Set the Start Time and Position of each object
        (Variables|Default|SetStartTime (Utilities|Time|GetRealTimeSeconds))
        (for (_array_element _array_index) (Variables|Default|GetObjects%20In%20BP)
          (Utilities|Array|SetArrayElem (Variables|Default|GetObjectsStartTransform) _array_index (Transformation|GetWorldTransform _array_element)))
        (Variables|/Game/FirstPersonCPP/Blueprints/FirstPersonCharacter.FirstPersonCharacter_C|SetbEnergyDecayingBP _player true)
        (Variables|/Game/FirstPersonCPP/Blueprints/FirstPersonCharacter.FirstPersonCharacter_C|SetbEnergyRegeneratingBP _player false))
      (else
        ;[1 1 1] If the object has been buit do nothing
        (if (not (Variables|Default|GetIsObjectBuilt))
          (for _array_element_2 (Variables|Default|GetObjects%20In%20BP)
            (Physics|SetSimulatePhysics _array_element_2 true)
            (Variables|/Game/FirstPersonCPP/Blueprints/FirstPersonCharacter.FirstPersonCharacter_C|SetbEnergyDecayingBP _player_2 false)
            (Variables|/Game/FirstPersonCPP/Blueprints/FirstPersonCharacter.FirstPersonCharacter_C|SetbEnergyRegeneratingBP _player_2 true)))))))

(event EventBeginPlay
  (bind _output_get (Variables|Default|SetPlayer (.AsFirst%20Person%20Character (Utilities|Casting|CastToFirstPersonCharacter (Game|GetPlayerCharacter 0)))))
  (EventDispatchers|BindEventtoDispatchtoReagableObjects _output_get (delegate Custom|PressButton))
  ;[1 1 1] This Changes Depending On the Number Of Components
  (Variables|Default|SetObjects%20In%20BP (Utilities|Array|MakeArray (Variables|Default|GetCylinder) (Variables|Default|GetCylinder1) (Variables|Default|GetCylinder2) (Variables|Default|GetCone)))
  (for (_array_element _array_index) (Variables|Default|GetObjects%20In%20BP)
    ;[1 1 1] set each end position
    (Utilities|Array|SetArrayElem (Variables|Default|GetBPObjectsTransforms) _array_index (Transformation|GetWorldTransform _array_element))
    ;[1 1 1] Move Each Component to a new position
    (Transformation|SetWorldTransform _array_element (Math|Transform|MakeTransform (Transformation|GetActorLocation (Utilities|Array|Get(acopy) (Variables|Default|GetStartTargetArray) _array_index)) (Math|Rotator|Lerp(Rotator) "270.000000,270.000000,270.000000" "90.000000,90.000000,90.000000" (Math|Random|RandomFloatinRange 0.0 1.0)) "1,1,1") false false)))

(event EventTick
  (params (DeltaSeconds :type Float%20%28single-precision%29))
  (bind _player (Variables|Default|GetPlayer))
  (bind _player_2 (Variables|Default|GetPlayer))
  (bind _player_3 (Variables|Default|GetPlayer))
  (bind _button (Variables|Default|GetButton))
  (bind _traveltime (Variables|Default|GetTravelTime))
  (bind _alpha (Utilities|CalculateAlpha _traveltime))
  (if (not (Variables|Default|GetIsObjectBuilt))
    ;[1 1 1] Is the player in the area
    (if (Variables|/Game/FirstPersonCPP/Blueprints/FirstPersonCharacter.FirstPersonCharacter_C|GetbInterationPressedBP (Variables|Default|GetPlayer))
      (Utilities|IsValid (Variables|/Game/FirstPersonCPP/Blueprints/FirstPersonCharacter.FirstPersonCharacter_C|GetLineTraceCompHitBP (Variables|Default|GetPlayer))
        (:Is%20Valid
          (if (== (Variables|/Game/FirstPersonCPP/Blueprints/FirstPersonCharacter.FirstPersonCharacter_C|GetLineTraceActorHitBP (Variables|Default|GetPlayer)) self)
            (if (<= (Variables|/Game/FirstPersonCPP/Blueprints/FirstPersonCharacter.FirstPersonCharacter_C|GetPlayer%20EnergyBP (Variables|Default|GetPlayer)) 0.0)
              ;[1 1 1] If the object has been buit do nothing
              (if (not (Variables|Default|GetIsObjectBuilt)) :!label _label
                (for _array_element (Variables|Default|GetObjects%20In%20BP)
                  (Physics|SetSimulatePhysics _array_element true)
                  (Variables|/Game/FirstPersonCPP/Blueprints/FirstPersonCharacter.FirstPersonCharacter_C|SetbEnergyDecayingBP _player_3 false)
                  (Variables|/Game/FirstPersonCPP/Blueprints/FirstPersonCharacter.FirstPersonCharacter_C|SetbEnergyRegeneratingBP _player_3 true)))
              (else
                ;[1 1 1] For each Component
                (for (_array_element_2 _array_index) (Variables|Default|GetObjects%20In%20BP)
                  (Variables|Default|SetArrayElement _array_element_2)
                  (Variables|Default|SetArrayIndex _array_index)
                  ;[1 1 1] Turn Off Physics
                  (Physics|SetSimulatePhysics (Variables|Default|GetArrayElement) false)
                  ;[1 1 1] Calculate teh Alpha
                  (if (>= _alpha 1.0)
                    (Variables|Default|SetAlpha 1.0)
                    (Variables|Default|SetIsObjectBuilt true)
                    (Variables|/Game/FirstPersonCPP/Blueprints/FirstPersonCharacter.FirstPersonCharacter_C|SetbEnergyDecayingBP _player_2 false)
                    (Variables|/Game/FirstPersonCPP/Blueprints/FirstPersonCharacter.FirstPersonCharacter_C|SetbEnergyRegeneratingBP _player_2 true)
                    (Utilities|Array|RemoveItem (Variables|/Script/Engine.ActorComponent|GetComponentTags (Variables|Default|GetButton)) "ReageableButton")
                    (Widget|RemovefromParent (Variables|/Game/FirstPersonCPP/Blueprints/FirstPersonCharacter.FirstPersonCharacter_C|GetInteractionQueHUD (Variables|Default|GetPlayer)))
                    (Variables|/Game/FirstPersonCPP/Blueprints/FirstPersonCharacter.FirstPersonCharacter_C|SetbInteractionQueHudVisableBP (Variables|Default|GetPlayer) false)
                    ;[1 1 1] Set the Transform of the component
                    (Transformation|SetWorldTransform (Variables|Default|GetArrayElement) (Math|Transform|Lerp(Transform) (Utilities|Array|Get(acopy) (Variables|Default|GetObjectsStartTransform) (Variables|Default|GetArrayIndex)) (Utilities|Array|Get(acopy) (Variables|Default|GetBPObjectsTransforms) (Variables|Default|GetArrayIndex)) (Variables|Default|GetAlpha)) false false :!label _label_2)
                    (else
                      (Variables|Default|SetAlpha _alpha)
                      (for _array_element_3 (Variables|Default|GetObjects%20In%20BP)
                        (bind _returnvalue (Rendering|Material|CreateDynamicMaterialInstance _array_element_3 0 (Rendering|Material|GetMaterial _array_element_3 0) :!class /Script/Engine.PrimitiveComponent))
                        (Rendering|Material|SetScalarParameterValue _returnvalue "Blend" (Variables|Default|GetAlpha) :!class /Script/Engine.MaterialInstanceDynamic)
                        (bind _returnvalue_2 (Rendering|Material|CreateDynamicMaterialInstance _button 0 (Rendering|Material|GetMaterial _button 0) :!class /Script/Engine.PrimitiveComponent))
                        (Rendering|Material|SetScalarParameterValue _returnvalue_2 "Blend" (Variables|Default|GetAlpha) :!class /Script/Engine.MaterialInstanceDynamic)
                        (goto _label_2)))))))
            (elif (not (Utilities|Array|ContainsItem (Variables|/Script/Engine.ActorComponent|GetComponentTags (Variables|/Game/FirstPersonCPP/Blueprints/FirstPersonCharacter.FirstPersonCharacter_C|GetLineTraceCompHitBP (Variables|Default|GetPlayer))) "ReageableButton"))
              (goto _label))))
        (:Is%20Not%20Valid
          (for _array_element_4 (Variables|Default|GetObjects%20In%20BP)
            (Physics|SetSimulatePhysics _array_element_4 true)
            (Variables|/Game/FirstPersonCPP/Blueprints/FirstPersonCharacter.FirstPersonCharacter_C|SetbEnergyDecayingBP _player false)
            (Variables|/Game/FirstPersonCPP/Blueprints/FirstPersonCharacter.FirstPersonCharacter_C|SetbEnergyRegeneratingBP _player true)))))))

(fn ConstructionScript)

(fn GetNewObjectTransform
  (params (Object%20To%20Move :type Static%20Mesh%20Component%20Object%20Reference) (TargetTransform :type Transform) (Speed :type Float%20%28single-precision%29))
  (bind _returnvalue (Transformation|GetWorldTransform Object%20To%20Move))
  (bind (_location _rotation _scale) (Math|Transform|BreakTransform _returnvalue))
  (return (Math|Transform|MakeTransform (+ (* (Math|Vector|Normalize (Class|KismetMathLibrary|GetDirectionVector (Transformation|GetWorldLocation Object%20To%20Move) (.Location (Math|Transform|BreakTransform TargetTransform)))) (* (Utilities|Time|GetWorldDeltaSeconds) Speed)) _location) _rotation _scale)))