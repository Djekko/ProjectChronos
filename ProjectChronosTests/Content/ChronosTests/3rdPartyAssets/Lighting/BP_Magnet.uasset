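; BP_Magnet is an actor that continuously spins its Mag1 component around the yaw axis, with the direction controlled by the player's reverse input.
; It caches the player as a FirstPersonCharacter on BeginPlay and polls ReverseButtonPressed every Tick.
; Yaw changes at a constant, delta-time-scaled rate, running backwards while that flag is set, with no recorded history.
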(event EventTick
  (params (DeltaSeconds :type Float%20%28single-precision%29))
  (bind _returnvalue (* DeltaSeconds 3e+01))
  (bind _mag1 (Variables|Default|GetMag1))
  (bind _relativerotation (Variables|/Script/Engine.SceneComponent|GetRelativeRotation _mag1))
  (if (Variables|/Script/ProjectChronosTests.ProjectChronosTestsCharacter|GetbReverseButtonPressed (Variables|Default|GetPlayer))
    (Transformation|SetRelativeRotation (Variables|Default|GetMag1) (Math|Rotator|MakeRotator (.roll _relativerotation) (.pitch _relativerotation) (- (.yaw _relativerotation) _returnvalue)) false false)
    (else
      (Transformation|SetRelativeRotation (Variables|Default|GetMag1) (Math|Rotator|MakeRotator (.roll _relativerotation) (.pitch _relativerotation) (+ (.yaw _relativerotation) _returnvalue)) false false))))

(event EventBeginPlay
  (Variables|Default|SetPlayer (.AsFirst%20Person%20Character (Utilities|Casting|CastToFirstPersonCharacter (Game|GetPlayerCharacter 0)))))

(fn ConstructionScript)