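; A vent light Blueprint that can flicker on and off at irregular intervals.
; When Flicker is set, Tick accumulates time and, on reaching the interval, picks a new random one between MinTime and MaxTime.
; A FlipFlop then toggles the point light intensity and swaps the Lightround mesh between a plain floor material and an emissive vent material, so glow matches light.
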(event EventTick
  (params (DeltaSeconds :type Float%20%28single-precision%29))
  (if (Variables|Default|GetFlicker)
    (bind _output_get (Variables|Default|SetTimePassedSinceLastChange (+ (Variables|Default|GetTimePassedSinceLastChange) DeltaSeconds)))
    (if (>= _output_get (Variables|Default|GetNextTime))
      (Variables|Default|SetTimePassedSinceLastChange 0.0)
      (Variables|Default|SetNextTime (Math|Random|RandomFloatinRange (Variables|Default|GetMinTime) (Variables|Default|GetMaxTime)))
      (Utilities|FlowControl|FlipFlop
        (:A
          (Rendering|Components|Light|SetIntensity (Variables|Default|GetPointLight) 0.0)
          (Rendering|Material|SetMaterial (Variables|Default|Getlight-round) 0 "/Game/StarterContent/Materials/M_Basic_Floor.M_Basic_Floor"))
        (:B
          (Rendering|Components|Light|SetIntensity (Variables|Default|GetPointLight) 1e+01)
          (Rendering|Material|SetMaterial (Variables|Default|Getlight-round) 0 "/Game/StarterContent/Materials/M_EmissiveLight_VENTS.M_EmissiveLight_VENTS"))))))

(fn ConstructionScript)