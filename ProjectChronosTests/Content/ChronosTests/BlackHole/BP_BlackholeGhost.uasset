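; BP_BlackholeGhost is a ghost actor for the black hole, intended to stay in front of the first-person player.
; It caches the player character on BeginPlay and moves its root every Tick to the result of GhostLocation.
; GhostLocation holds math projecting the player's BlackholeDistFromPlayer along the camera's forward vector, though that expression appears unconnected to any output.
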(event EventTick
  (params (DeltaSeconds :type Float%20%28single-precision%29))
  ;[1 1 1] Set the Position to Always Be Infront of the Player
  (Transformation|SetWorldLocation (Variables|Default|GetDefaultSceneRoot) (Utilities|GhostLocation) false false))

(event EventBeginPlay
  ;[1 1 1] Get Player Ref
  (Variables|Default|SetPlayer (.AsFirst%20Person%20Character (Utilities|Casting|CastToFirstPersonCharacter (Game|GetPlayerCharacter 0)))))

(fn ConstructionScript)