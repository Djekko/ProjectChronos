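; Black hole actor that scales with a timeline, pulls in overlapping components and destroys non-exempt actors touching its core.
; GlassAOE disables gravity and blocking, adds spin and a collapse material, and restores physics on exit; Tick moves components toward SphereX.
; For time rewind, toggling the player's reverse state reverses the timeline, and normal expiry logs the actor's class, time and transform on the player.
; Player-carry and distance-based shrink logic are disconnected.
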(event OnComponentBeginOverlap(SphereX)
  (params (OverlappedComponent :type Primitive%20Component%20Object%20Reference) (OtherActor :type Actor%20Object%20Reference) (OtherComp :type Primitive%20Component%20Object%20Reference) (OtherBodyIndex :type Integer) (bFromSweep :type Boolean) (SweepResult :type Hit%20Result%20Structure%20%28by%20ref%29))
  ;[0 1 0.2456] Comment
  (Variables|Default|SetBlackHoleOverlappedActor OtherActor)
  (Variables|Default|SetBlackHoleOverlappedComp OtherComp)
  ;;[1 1 1] is the overlapped actor itself
  (if (not (== (Variables|Default|GetBlackHoleOverlappedActor) self))
    ;;[1 1 1] Is the Comp Singularity Exempt
    (if (not (Utilities|IsSingularityExempt (Variables|Default|GetBlackHoleOverlappedComp)))
      (Actor|DestroyActor (Variables|Default|GetBlackHoleOverlappedActor)))))

(event OnComponentBeginOverlap(GlassAOE)
  (params (OverlappedComponent :type Primitive%20Component%20Object%20Reference) (OtherActor :type Actor%20Object%20Reference) (OtherComp :type Primitive%20Component%20Object%20Reference) (OtherBodyIndex :type Integer) (bFromSweep :type Boolean) (SweepResult :type Hit%20Result%20Structure%20%28by%20ref%29))
  (bind _returnvalue (Math|Random|RandomFloatinRange -3.6e+02 3.6e+02))
  (bind _spherex (Variables|Default|GetSphereX))
  (bind _returnvalue_2 (Transformation|GetWorldLocation _spherex))
  ;[0 1 0.2456] Comment
  (Variables|Default|SetAOEOverlappingComp OtherComp)
  ;;[1 1 1] Is the Comp Exempt from effects
  (if (not (Utilities|IsSingularityExempt (Variables|Default|GetAOEOverlappingComp)))
    ;;[1 1 1] Turn Off Gravity and allow to overlap other components
    (Physics|SetEnableGravity (Variables|Default|GetAOEOverlappingComp) false)
    (Collision|SetCollisionResponsetoAllChannels (Variables|Default|GetAOEOverlappingComp) "ECR_Overlap")
    ;;[1 1 1] Give the comp a random rotation
    (Class|PrimitiveComponent|SetPhysicsAngularVelocity (Variables|Default|GetAOEOverlappingComp) (Math|Vector|MakeVector _returnvalue _returnvalue _returnvalue) false "None")
    (Rendering|Material|SetMaterial (Variables|Default|GetAOEOverlappingComp) 0 "/Game/ChronosTests/BlackHole/VFX/Materials/M_VolumeSphereMaster2.M_VolumeSphereMaster2")
    (bind _returnvalue_3 (Rendering|Material|CreateDynamicMaterialInstance (Variables|Default|GetAOEOverlappingComp) 0 (Rendering|Material|GetMaterial (Variables|Default|GetAOEOverlappingComp) 0) :!class /Script/Engine.PrimitiveComponent))
    (Rendering|Material|SetVectorParameterValue _returnvalue_3 "CollapseLocation" (Utilities|Struct|MakeLinearColor (.x _returnvalue_2) (.y _returnvalue_2) (.z _returnvalue_2) 0.0) :!class /Script/Engine.MaterialInstanceDynamic)))

(event OnComponentEndOverlap(GlassAOE)
  (params (OverlappedComponent :type Primitive%20Component%20Object%20Reference) (OtherActor :type Actor%20Object%20Reference) (OtherComp :type Primitive%20Component%20Object%20Reference) (OtherBodyIndex :type Integer))
  ;[0 1 0.2456] Comment
  (Variables|Default|SetAOEEndOverlappedComp OtherComp)
  ;;[1 1 1] Is the Comp Exempt from effects
  (if (not (Utilities|IsSingularityExempt (Variables|Default|GetAOEEndOverlappedComp)))
    ;;[1 1 1] Give Comp gravity collisions and the correct scale
    (Physics|SetEnableGravity (Variables|Default|GetAOEEndOverlappedComp) true)
    (Collision|SetCollisionResponsetoAllChannels (Variables|Default|GetAOEEndOverlappedComp) "ECR_Block")
    (Transformation|SetWorldScale3D (Variables|Default|GetAOEEndOverlappedComp) "1.000000,1.000000,1.000000")))

(event Custom|ReverseBlackHole
  ;[0 1 0.2445] Comment
  ;;[1 1 1] make tha scale 0 and then incread to give the illusion of expanding
  (bind _singularityscale (Timeline|SingularityExpand Reverse)
    (:Update
      (Transformation|SetActorScale3D self _singularityscale))
    (:Finished
      (if (Variables|Default|GetReversing%20BlackholeBP)
        (Actor|DestroyActor self :!label _label)
        (elif (Variables|Default|GetSpawnedReversingBP)
          (goto _label)
          (else
            ;;;[0 0.19 1] MoreRewindStuff
            (Utilities|Array|Add (Variables|/Game/FirstPersonCPP/Blueprints/FirstPersonCharacter.FirstPersonCharacter_C|GetActorDestroyedBP (Variables|Default|GetPlayer)) "BP_BlackHoleParticals_C")
            (Utilities|Array|Add (Variables|/Game/FirstPersonCPP/Blueprints/FirstPersonCharacter.FirstPersonCharacter_C|GetDestroyed%20timeBP (Variables|Default|GetPlayer)) (Utilities|Time|GetRealTimeSeconds))
            (Utilities|Array|Add (Variables|/Game/FirstPersonCPP/Blueprints/FirstPersonCharacter.FirstPersonCharacter_C|GetDestroyedTransformBP (Variables|Default|GetPlayer)) (Transformation|GetActorTransform self))
            (Actor|DestroyActor self)))))))

(event EventTick
  (params (DeltaSeconds :type Float%20%28single-precision%29))
  ;[0 1 0.1392] Comment
  ;;[0.03732 0.05826 0.415] RewindStuff
  (if (Variables|Default|GetSpawnedReversingBP)
    (if (Variables|/Script/ProjectChronosTests.ProjectChronosTestsCharacter|GetbReverseButtonPressed (Variables|Default|GetPlayer))
      _
      (else
        (if (Variables|Default|GetReversing%20BlackholeBP) :!label _label
          _
          (else
            (Variables|Default|SetReversing%20BlackholeBP true)
            (CallFunction|ReverseBlackHole)))))
    (elif (Variables|/Script/ProjectChronosTests.ProjectChronosTestsCharacter|GetbReverseButtonPressed (Variables|Default|GetPlayer))
      (goto _label)
      (else
        _)))
  ;;[1 1 1] For each Object In the AoE
  (for _array_element (Class|PrimitiveComponent|GetOverlappingComponents (Variables|Default|GetGlassAOE))
    (Variables|Default|SetArrayElement _array_element)
    ;;[1 1 1] If the Element Is Itslef
    (if (not (== (Components|GetOwner (Variables|Default|GetArrayElement)) self))
      ;;[1 1 1] If target is exempt of the blackhole
      (if (not (Utilities|Array|ContainsItem (Variables|/Script/Engine.ActorComponent|GetComponentTags (Variables|Default|GetArrayElement)) "SingularityExempt"))
        ;;[1 1 1] Set New Array Elemnt Transform
        (bind _newobjecttransform (CallFunction|GetNewObjectTransform (Variables|Default|GetArrayElement) (Variables|Default|GetSphereX) (Variables|Default|GetSpeedBP)))
        (Transformation|SetWorldTransform (Variables|Default|GetArrayElement) _newobjecttransform false false)))))

(event EventBeginPlay
  ;[0 1 0.2445] Comment
  ;;[1 1 1] Make This Actor TimeExmpt
  (Utilities|Array|Add (Variables|Actor|GetTags self) "TimeExempt")
  ;;[1 1 1] GetPlayerRef
  (Variables|Default|SetPlayer (.AsFirst%20Person%20Character (Utilities|Casting|CastToFirstPersonCharacter (Game|GetPlayerCharacter 0))))
  (if (Variables|/Script/ProjectChronosTests.ProjectChronosTestsCharacter|GetbReverseButtonPressed (Variables|Default|GetPlayer))
    ;;[0 0.118 1] RewindStuff
    (Variables|Default|SetSpawnedReversingBP true)
    ;;[1 1 1] make tha scale 0 and then incread to give the illusion of expanding
    (bind _singularityscale (Timeline|SingularityExpand PlayFromStart)
      (:Update
        (Transformation|SetActorScale3D self _singularityscale))
      (:Finished
        (if (Variables|Default|GetReversing%20BlackholeBP)
          (Actor|DestroyActor self :!label _label)
          (elif (Variables|Default|GetSpawnedReversingBP)
            (goto _label)
            (else
              ;;;[0 0.19 1] MoreRewindStuff
              (Utilities|Array|Add (Variables|/Game/FirstPersonCPP/Blueprints/FirstPersonCharacter.FirstPersonCharacter_C|GetActorDestroyedBP (Variables|Default|GetPlayer)) "BP_BlackHoleParticals_C")
              (Utilities|Array|Add (Variables|/Game/FirstPersonCPP/Blueprints/FirstPersonCharacter.FirstPersonCharacter_C|GetDestroyed%20timeBP (Variables|Default|GetPlayer)) (Utilities|Time|GetRealTimeSeconds))
              (Utilities|Array|Add (Variables|/Game/FirstPersonCPP/Blueprints/FirstPersonCharacter.FirstPersonCharacter_C|GetDestroyedTransformBP (Variables|Default|GetPlayer)) (Transformation|GetActorTransform self))
              (Actor|DestroyActor self))))))
    (else
      (Variables|Default|SetSpawnedReversingBP false)
      (Timeline|SingularityExpand PlayFromStart))))

(fn ConstructionScript)

(fn GetNewObjectTransform
  (params (ObjectToMove :type Primitive%20Component%20Object%20Reference) (ObjectTarget :type Static%20Mesh%20Component%20Object%20Reference) (Speed :type Float%20%28single-precision%29))
  (bind _returnvalue (Transformation|GetWorldTransform ObjectToMove))
  (bind (_location _rotation _scale) (Math|Transform|BreakTransform _returnvalue))
  (return (Math|Transform|MakeTransform (+ (* (Math|Vector|Normalize (Class|KismetMathLibrary|GetDirectionVector (Transformation|GetWorldLocation ObjectToMove) (Transformation|GetWorldLocation ObjectTarget))) (* (Utilities|Time|GetWorldDeltaSeconds) Speed)) _location) _rotation _scale)))

(fn GetNewObjectScale
  (params (ObjectToScale :type Primitive%20Component%20Object%20Reference))
  (LocalVariables|SetObject ObjectToScale)
  (if (> (/ (* (Math|Vector|VectorLength (- (Transformation|GetWorldLocation (Variables|Default|GetSphereX)) (Transformation|GetWorldLocation (LocalVariables|GetObject)))) (/ 1e+02 3.4e+02)) 1e+02) 1.0)
    (LocalVariables|SetNewObScale "1.000000,1.000000,1.000000")
    (else
      (LocalVariables|SetNewObScale (Math|Vector|MakeVector (/ (* (Math|Vector|VectorLength (- (Transformation|GetWorldLocation (Variables|Default|GetSphereX)) (Transformation|GetWorldLocation (LocalVariables|GetObject)))) (/ 1e+02 3.4e+02)) 1e+02) (/ (* (Math|Vector|VectorLength (- (Transformation|GetWorldLocation (Variables|Default|GetSphereX)) (Transformation|GetWorldLocation (LocalVariables|GetObject)))) (/ 1e+02 3.4e+02)) 1e+02) (/ (* (Math|Vector|VectorLength (- (Transformation|GetWorldLocation (Variables|Default|GetSphereX)) (Transformation|GetWorldLocation (LocalVariables|GetObject)))) (/ 1e+02 3.4e+02)) 1e+02)))))
  (return (LocalVariables|GetNewObScale)))