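; BP_ShockWave is a shockwave actor that travels forward from its spawn point and supports the player's time rewind.
; One timeline drives its scale, material fade and position, running backward if it spawns while reverse is pressed.
; Tick flips the timeline direction once when the player's reverse state changes.
; An unreversed, forward-spawned wave logs its class, time and start transform to the player's destroyed-actor arrays before destroying itself.
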(event Custom|ReverseShockwave
  (bind _self self)
  (bind _returnvalue (Transformation|GetActorTransform _self))
  (if (Variables|Default|GetSpawnedReversingBP)
    (bind (_direction _fade _scale _distance_alpha) (Timeline|TL_ShockWave Play)
      (:Update
        (Rendering|Material|SetScalarParameterValueonMaterials (Variables|Default|GetShockWave) "ShockWaveFade" _fade)
        (Transformation|SetActorScale3D self (Math|Vector|MakeVector _scale _scale _scale))
        (Transformation|SetActorLocation self (Math|Vector|Lerp(Vector) (Variables|Default|GetShockWaveStartLocationBP) (Variables|Default|GetShockWaveEndLocationBP) _distance_alpha) false false))
      (:Finished
        ;[0 0.2118 1] TimeRewindStuff
        (if (Variables|Default|GetReversingShockWaveBP)
          (Actor|DestroyActor self :!label _label)
          (elif (Variables|Default|GetSpawnedReversingBP)
            (goto _label)
            (else
              (Utilities|Array|Add (Variables|/Game/FirstPersonCPP/Blueprints/FirstPersonCharacter.FirstPersonCharacter_C|GetActorDestroyedBP (Variables|Default|GetPlayer)) "BP_ShockWave_C")
              (Utilities|Array|Add (Variables|/Game/FirstPersonCPP/Blueprints/FirstPersonCharacter.FirstPersonCharacter_C|GetDestroyed%20timeBP (Variables|Default|GetPlayer)) (Utilities|Time|GetRealTimeSeconds))
              (Utilities|Array|Add (Variables|/Game/FirstPersonCPP/Blueprints/FirstPersonCharacter.FirstPersonCharacter_C|GetDestroyedTransformBP (Variables|Default|GetPlayer)) (Math|Transform|MakeTransform (Variables|Default|GetShockWaveStartLocationBP) (.rotation _returnvalue) (.scale _returnvalue)))
              (Actor|DestroyActor))))))
    (else
      (Timeline|TL_ShockWave Reverse))))

(event EventBeginPlay
  (bind _self self)
  (bind _self_2 self)
  (bind _self_3 self)
  (bind _returnvalue (Transformation|GetActorTransform _self_3))
  (Variables|Default|SetPlayer (.AsFirst%20Person%20Character (Utilities|Casting|CastToFirstPersonCharacter (Game|GetPlayerCharacter 0))))
  (Variables|Default|SetShockWaveEndLocationBP (+ (Transformation|GetActorLocation _self_2) (* (Math|Vector|GetForwardVector (Transformation|GetActorRotation _self_2)) 8e+02)))
  (Variables|Default|SetShockWaveStartLocationBP (+ (Transformation|GetActorLocation _self) (* (Math|Vector|GetForwardVector (Transformation|GetActorRotation _self)) 5e+01)))
  (if (Variables|/Script/ProjectChronosTests.ProjectChronosTestsCharacter|GetbReverseButtonPressed (Variables|Default|GetPlayer))
    (Variables|Default|SetSpawnedReversingBP true)
    (bind (_direction _fade _scale _distance_alpha) (Timeline|TL_ShockWave ReverseFromEnd)
      (:Update
        (Rendering|Material|SetScalarParameterValueonMaterials (Variables|Default|GetShockWave) "ShockWaveFade" _fade)
        (Transformation|SetActorScale3D self (Math|Vector|MakeVector _scale _scale _scale))
        (Transformation|SetActorLocation self (Math|Vector|Lerp(Vector) (Variables|Default|GetShockWaveStartLocationBP) (Variables|Default|GetShockWaveEndLocationBP) _distance_alpha) false false))
      (:Finished
        ;[0 0.2118 1] TimeRewindStuff
        (if (Variables|Default|GetReversingShockWaveBP)
          (Actor|DestroyActor self :!label _label)
          (elif (Variables|Default|GetSpawnedReversingBP)
            (goto _label)
            (else
              (Utilities|Array|Add (Variables|/Game/FirstPersonCPP/Blueprints/FirstPersonCharacter.FirstPersonCharacter_C|GetActorDestroyedBP (Variables|Default|GetPlayer)) "BP_ShockWave_C")
              (Utilities|Array|Add (Variables|/Game/FirstPersonCPP/Blueprints/FirstPersonCharacter.FirstPersonCharacter_C|GetDestroyed%20timeBP (Variables|Default|GetPlayer)) (Utilities|Time|GetRealTimeSeconds))
              (Utilities|Array|Add (Variables|/Game/FirstPersonCPP/Blueprints/FirstPersonCharacter.FirstPersonCharacter_C|GetDestroyedTransformBP (Variables|Default|GetPlayer)) (Math|Transform|MakeTransform (Variables|Default|GetShockWaveStartLocationBP) (.rotation _returnvalue) (.scale _returnvalue)))
              (Actor|DestroyActor))))))
    (else
      (Variables|Default|SetSpawnedReversingBP false)
      (Timeline|TL_ShockWave PlayFromStart))))

(event EventTick
  (params (DeltaSeconds :type Float%20%28single-precision%29))
  ;[0.03732 0.05826 0.415] RewindStuff
  (if (Variables|Default|GetSpawnedReversingBP)
    (if (not (Variables|/Script/ProjectChronosTests.ProjectChronosTestsCharacter|GetbReverseButtonPressed (Variables|Default|GetPlayer)))
      (if (not (Variables|Default|GetReversingShockWaveBP)) :!label _label
        (Variables|Default|SetReversingShockWaveBP true)
        (CallFunction|ReverseShockwave)))
    (elif (Variables|/Script/ProjectChronosTests.ProjectChronosTestsCharacter|GetbReverseButtonPressed (Variables|Default|GetPlayer))
      (goto _label))))

(fn ConstructionScript)