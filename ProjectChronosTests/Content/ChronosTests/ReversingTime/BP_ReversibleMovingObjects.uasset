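; Component that gives a physics-simulated static mesh reversible time, driven by the first-person character's reverse button.
; Each tick it records transforms and velocities in capped arrays, packing linear and angular velocity into a Transform's location and scale.
; While rewinding it pops these samples, negates velocities and pushes them to replay stacks.
; On release it flips velocity back and replays the rewound motion unless the BreakTimeReplay tag clears it.
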(event Custom|ReplayTrans
  (bind _returnvalue (Components|GetOwner))
  (bind _returnvalue_2 (Components|GetOwner))
  (bind _tags (Variables|/Script/Engine.Actor|GetTags _returnvalue))
  (bind _tags_2 (Variables|/Script/Engine.Actor|GetTags _returnvalue_2))
  ;[0.03736 1 0] Replay Movement Of Objects
  (if (Utilities|Array|ContainsItem _tags_2 "CanBreak")
    _
    (else
      (Utilities|Array|Add _tags_2 "CanBreak")))
  (if (Utilities|Array|ContainsItem (Variables|/Script/Engine.Actor|GetTags (Components|GetOwner)) "BreakTimeReplay")
    (Variables|Default|SetReplayTransformBP (Utilities|Array|MakeArray ""))
    (elif (> (Utilities|Array|LastIndex (Variables|Default|GetReplayTransformBP)) 0)
      (Transformation|SetWorldTransform (Variables|Default|GetOwner) (Utilities|Array|Get(acopy) (Variables|Default|GetReplayTransformBP) (Utilities|Array|LastIndex (Variables|Default|GetReplayTransformBP))) false false)
      (if (> (Utilities|Array|LastIndex (Variables|Default|GetReplayTransformBP)) 0)
        (Utilities|Array|RemoveIndex (Variables|Default|GetReplayTransformBP) (Utilities|Array|LastIndex (Variables|Default|GetReplayTransformBP))))
      (elif (Utilities|Array|ContainsItem _tags "CanBreak")
        (Utilities|Array|RemoveItem _tags "CanBreak")))))

(event Custom|ReplayVeloc
  ;[0.03736 1 0] Replay Movement Of Objects
  (if (Utilities|Array|ContainsItem (Variables|/Script/Engine.Actor|GetTags (Components|GetOwner)) "BreakTimeReplay")
    (Variables|Default|SetReplayVelocityBP (Utilities|Array|MakeArray ""))
    (elif (> (Utilities|Array|LastIndex (Variables|Default|GetReplayVelocityBP)) 0)
      (Physics|SetPhysicsLinearVelocity (Variables|Default|GetOwner) (.Location (Math|Transform|BreakTransform (Utilities|Array|Get(acopy) (Variables|Default|GetReplayVelocityBP) (Utilities|Array|LastIndex (Variables|Default|GetReplayVelocityBP))))) false "None")
      (Class|PrimitiveComponent|SetPhysicsAngularVelocity (Variables|Default|GetOwner) (.Scale (Math|Transform|BreakTransform (Utilities|Array|Get(acopy) (Variables|Default|GetReplayVelocityBP) (Utilities|Array|LastIndex (Variables|Default|GetReplayVelocityBP))))) false "None")
      (if (> (Utilities|Array|LastIndex (Variables|Default|GetReplayVelocityBP)) 0)
        (Utilities|Array|RemoveIndex (Variables|Default|GetReplayVelocityBP) (Utilities|Array|LastIndex (Variables|Default|GetReplayVelocityBP)))))))

(event EventTick
  (params (DeltaSeconds :type Float%20%28single-precision%29))
  (bind _characterreferance (Variables|Default|GetCharacterReferance))
  (bind _transformarraybp (Variables|Default|GetTransformArrayBP))
  (bind _transformarraybp_2 (Variables|Default|GetTransformArrayBP))
  (bind _velocityarraybp (Variables|Default|GetVelocityArrayBP))
  (bind _velocityarraybp_2 (Variables|Default|GetVelocityArrayBP))
  (bind _transformarraybp_3 (Variables|Default|GetTransformArrayBP))
  (bind _velocityarraybp_3 (Variables|Default|GetVelocityArrayBP))
  (bind _returnvalue (Utilities|Array|LastIndex _velocityarraybp))
  (bind _breversebuttonpressed (Variables|/Script/ProjectChronosTests.ProjectChronosTestsCharacter|GetbReverseButtonPressed _characterreferance))
  (bind _item (Utilities|Array|Get(acopy) _velocityarraybp _returnvalue))
  (bind (_location _rotation _scale) (Math|Transform|BreakTransform _item))
  ;[0.002349 1 0] Rewind Time
  (Utilities|FlowControl|Sequence
    (:then_0
      (if _breversebuttonpressed
        (Transformation|SetWorldTransform (Variables|Default|GetOwner) (Utilities|Array|Get(acopy) _transformarraybp_2 (Utilities|Array|LastIndex _transformarraybp_2)) false false)
        (if (> (Utilities|Array|LastIndex (Variables|Default|GetTransformArrayBP)) 0)
          ;;[1 1 1] storing values to replay what just happened
          (Utilities|Array|Add (Variables|Default|GetReplayTransformBP) (Utilities|Array|Get(acopy) _transformarraybp (Utilities|Array|LastIndex _transformarraybp)))
          (Utilities|Array|RemoveIndex (Variables|Default|GetTransformArrayBP) (Utilities|Array|LastIndex (Variables|Default|GetTransformArrayBP))))
        (else
          (if (>= (Utilities|Array|Length _transformarraybp_3) (Variables|Default|GetMaximumArrayLengthBP))
            (Utilities|Array|RemoveIndex _transformarraybp_3))
          (Utilities|Array|Add (Variables|Default|GetTransformArrayBP) (Transformation|GetWorldTransform (Variables|Default|GetOwner)))
          (CallFunction|ReplayTrans))))
    (:then_1
      (if _breversebuttonpressed
        (Variables|Default|SetResetVelocityBP true)
        (Physics|SetPhysicsLinearVelocity (Variables|Default|GetOwner) (* _location -1.0) false "None")
        (Class|PrimitiveComponent|SetPhysicsAngularVelocity (Variables|Default|GetOwner) (* _scale -1.0) false "None")
        (if (> (Utilities|Array|LastIndex (Variables|Default|GetVelocityArrayBP)) 0)
          ;;[1 1 1] storing values to replay what just happened
          (Utilities|Array|Add (Variables|Default|GetReplayVelocityBP) (Utilities|Array|Get(acopy) _velocityarraybp_2 (Utilities|Array|LastIndex _velocityarraybp_2)))
          (Utilities|Array|RemoveIndex (Variables|Default|GetVelocityArrayBP) (Utilities|Array|LastIndex (Variables|Default|GetVelocityArrayBP))))
        (else
          ;;[1 0.08185 0.1316] Reset The Reverse Velocity So the object moves in the right direction
          (if (Variables|Default|GetResetVelocityBP)
            (bind _returnvalue_2 (Physics|GetPhysicsLinearVelocity (Variables|Default|GetOwner) "None"))
            (Physics|SetPhysicsLinearVelocity (Variables|Default|GetOwner) (* _returnvalue_2 -1.0) false "None")
            (bind _returnvalue_3 (Class|PrimitiveComponent|GetPhysicsAngularVelocity (Variables|Default|GetOwner) "None"))
            (Class|PrimitiveComponent|SetPhysicsAngularVelocity (Variables|Default|GetOwner) (* _returnvalue_3 -1.0) false "None")
            (Variables|Default|SetResetVelocityBP false))
          ;;[1 1 1] delete elements from the start of the array if it is too long
          (if (>= (Utilities|Array|Length _velocityarraybp_3) (Variables|Default|GetMaximumArrayLengthBP))
            (Utilities|Array|RemoveIndex _velocityarraybp_3))
          (CallFunction|ReplayVeloc)
          (bind _returnvalue_4 (Class|PrimitiveComponent|GetPhysicsAngularVelocity (Variables|Default|GetOwner) "None"))
          (bind _returnvalue_5 (Physics|GetPhysicsLinearVelocity (Variables|Default|GetOwner) "None"))
          (Utilities|Array|Add (Variables|Default|GetVelocityArrayBP) (Math|Transform|MakeTransform _returnvalue_5 "0, 0, 0" _returnvalue_4)))))))

(event EventBeginPlay
  ;[0.07241 1 0] Comment
  (Utilities|Array|Add (Variables|/Script/Engine.Actor|GetTags (Components|GetOwner)) "ReveraibleObject")
  ;;[1 1 1] get player ref
  (Variables|Default|SetCharacterReferance (.AsFirst%20Person%20Character (Utilities|Casting|CastToFirstPersonCharacter (Game|GetPlayerCharacter 0))))
  ;;[1 1 1] Get the Owner of this comp
  (bind _output_get (Variables|Default|SetOwner (Utilities|Array|Get(acopy) (Actor|GetComponentsByClass (Components|GetOwner self) "/Script/Engine.StaticMeshComponent"))))
  (Variables|/Script/Engine.PrimitiveComponent|SetbGenerateOverlapEvents _output_get true)
  (Physics|SetSimulatePhysics (Variables|Default|GetOwner) true))