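; Component that lets its owning actor's first static mesh, with physics simulation off, rewind through time and replay the undone movement.
; Each tick it records the mesh transform into a capped history, or pops that history while the player holds reverse.
; Rewound transforms go onto a replay stack, played back once reverse is released.
; Actor tags coordinate this: CanBreak marks replay in progress, and BreakTimeReplay discards the stack.
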(event Custom|ReplayTrans
  (bind _returnvalue (Components|GetOwner))
  (bind _returnvalue_2 (Components|GetOwner))
  (bind _tags (Variables|/Script/Engine.Actor|GetTags _returnvalue))
  (bind _tags_2 (Variables|/Script/Engine.Actor|GetTags _returnvalue_2))
  ;[1 1 1] Replay Movement Of Objects
  (if (Utilities|Array|ContainsItem _tags_2 "CanBreak")
    _
    (else
      (Utilities|Array|Add _tags_2 "CanBreak")))
  (if (Utilities|Array|ContainsItem (Variables|/Script/Engine.Actor|GetTags (Components|GetOwner)) "BreakTimeReplay")
    (Variables|Default|SetReplayTransform (Utilities|Array|MakeArray ""))
    (elif (> (Utilities|Array|LastIndex (Variables|Default|GetReplayTransform)) 0)
      (Transformation|SetWorldTransform (Variables|Default|GetOwner) (Utilities|Array|Get(acopy) (Variables|Default|GetReplayTransform) (Utilities|Array|LastIndex (Variables|Default|GetReplayTransform))) false false)
      (if (> (Utilities|Array|LastIndex (Variables|Default|GetReplayTransform)) 0)
        (Utilities|Array|RemoveIndex (Variables|Default|GetReplayTransform) (Utilities|Array|LastIndex (Variables|Default|GetReplayTransform))))
      (elif (Utilities|Array|ContainsItem _tags "CanBreak")
        (Utilities|Array|RemoveItem _tags "CanBreak")))))

(event EventTick
  (params (DeltaSeconds :type Float%20%28single-precision%29))
  (bind _transformarray (Variables|Default|GetTransformArray))
  (bind _transformarray_2 (Variables|Default|GetTransformArray))
  (bind _transformarray_3 (Variables|Default|GetTransformArray))
  ;[1 1 1] Rewind Time
  (if (Variables|/Script/ProjectChronosTests.ProjectChronosTestsCharacter|GetbReverseButtonPressed (Variables|Default|GetCharacterReferance))
    (Transformation|SetWorldTransform (Variables|Default|GetOwner) (Utilities|Array|Get(acopy) _transformarray_2 (Utilities|Array|LastIndex _transformarray_2)) false false)
    (if (> (Utilities|Array|LastIndex (Variables|Default|GetTransformArray)) 0)
      ;;[1 1 1] storing values to replay what just happened
      (Utilities|Array|Add (Variables|Default|GetReplayTransform) (Utilities|Array|Get(acopy) _transformarray (Utilities|Array|LastIndex _transformarray)))
      (Utilities|Array|RemoveIndex (Variables|Default|GetTransformArray) (Utilities|Array|LastIndex (Variables|Default|GetTransformArray))))
    (else
      (if (>= (Utilities|Array|Length _transformarray_3) (Variables|Default|GetMaximumArrayLength))
        (Utilities|Array|RemoveIndex _transformarray_3))
      (Utilities|Array|Add (Variables|Default|GetTransformArray) (Transformation|GetWorldTransform (Variables|Default|GetOwner)))
      (CallFunction|ReplayTrans))))

(event EventBeginPlay
  (Utilities|Array|Add (Variables|/Script/Engine.Actor|GetTags (Components|GetOwner)) "ReveraibleObject")
  ;[1 1 1] get player ref
  (Variables|Default|SetCharacterReferance (.AsFirst%20Person%20Character (Utilities|Casting|CastToFirstPersonCharacter (Game|GetPlayerCharacter 0))))
  ;[1 1 1] Get the Owner of this comp
  (bind _output_get (Variables|Default|SetOwner (Utilities|Array|Get(acopy) (Actor|GetComponentsByClass (Components|GetOwner self) "/Script/Engine.StaticMeshComponent"))))
  (Variables|/Script/Engine.PrimitiveComponent|SetbGenerateOverlapEvents _output_get true)
  (Physics|SetSimulatePhysics (Variables|Default|GetOwner) false))