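; BP_ReverseTimeEnergy is an overlap pickup that adds time energy to the first-person player for the time-reversal test.
; On BeginPlay it caches the FirstPersonCharacter.
; Cube overlaps from non-StaticMeshComponent components increment the player's energy count, unless the reverse button is pressed or the cap of three is reached.
; Its DestroyActor call is unconnected, so the actor persists and can grant energy again.
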(event OnComponentBeginOverlap(Cube)
  (params (OverlappedComponent :type Primitive%20Component%20Object%20Reference) (OtherActor :type Actor%20Object%20Reference) (OtherComp :type Primitive%20Component%20Object%20Reference) (OtherBodyIndex :type Integer) (bFromSweep :type Boolean) (SweepResult :type Hit%20Result%20Structure%20%28by%20ref%29))
  (if (not (== (Utilities|GetClass OtherComp) "/Script/Engine.StaticMeshComponent"))
    (if (not (Variables|/Script/ProjectChronosTests.ProjectChronosTestsCharacter|GetbReverseButtonPressed (Variables|Default|GetPlayer)))
      (if (not (>= (Variables|/Game/FirstPersonCPP/Blueprints/FirstPersonCharacter.FirstPersonCharacter_C|GetNumOfTimeEnergyBP (Variables|Default|GetPlayer)) 3))
        (Math|Integer|IncrementInt (Variables|/Game/FirstPersonCPP/Blueprints/FirstPersonCharacter.FirstPersonCharacter_C|GetNumOfTimeEnergyBP (Variables|Default|GetPlayer)))))))

(event EventBeginPlay
  (Variables|Default|SetPlayer (.AsFirst%20Person%20Character (Utilities|Casting|CastToFirstPersonCharacter (Game|GetPlayerCharacter 0)))))

(fn ConstructionScript)