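; Climbable ladder actor that extends itself downward and toggles the first-person player's climbing state.
; On BeginPlay, a short downward trace that hits nothing spawns another segment at the Arrow and destroys its own LadderBox, recursively leaving only the last segment's trigger.
; Overlapping that box exits climbing to Walking, or, if the player faces the ladder, enters Flying while a timeline aligns the capsule horizontally and turns it toward the ladder.
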(event OnComponentBeginOverlap(LadderBox)
  (params (OverlappedComponent :type Primitive%20Component%20Object%20Reference) (OtherActor :type Actor%20Object%20Reference) (OtherComp :type Primitive%20Component%20Object%20Reference) (OtherBodyIndex :type Integer) (bFromSweep :type Boolean) (SweepResult :type Hit%20Result%20Structure%20%28by%20ref%29))
  (bind _player (Variables|Default|GetPlayer))
  (bind _player_2 (Variables|Default|GetPlayer))
  (bind _defaultsceneroot (Variables|Default|GetDefaultSceneRoot))
  (bind _arrow1 (Variables|Default|GetArrow1))
  (bind _player_3 (Variables|Default|GetPlayer))
  (bind _returnvalue (Transformation|GetWorldLocation _arrow1))
  (bind _returnvalue_2 (Transformation|GetWorldLocation _defaultsceneroot))
  (bind _capsulecomponent (Variables|/Script/Engine.Character|GetCapsuleComponent _player_2))
  (bind _capsulecomponent_2 (Variables|/Script/Engine.Character|GetCapsuleComponent _player))
  (bind _capsulecomponent_3 (Variables|/Script/Engine.Character|GetCapsuleComponent _player_3))
  (bind _returnvalue_3 (Transformation|GetWorldLocation _capsulecomponent_2))
  (bind _returnvalue_4 (Transformation|GetWorldLocation _capsulecomponent_3))
  (if (== (Variables|/Script/Engine.Character|GetCapsuleComponent (Variables|Default|GetPlayer)) OtherComp)
    (if (Variables|/Script/ProjectChronosTests.ProjectChronosTestsCharacter|GetbCanClimbLadder (Variables|Default|GetPlayer))
      (Variables|/Script/ProjectChronosTests.ProjectChronosTestsCharacter|SetbCanClimbLadder (Variables|Default|GetPlayer) false)
      (Pawn|Components|CharacterMovement|SetMovementMode (Variables|/Script/Engine.Character|GetCharacterMovement (Variables|Default|GetPlayer)) "MOVE_Walking" 0)
      (elif (Variables|/Script/ProjectChronosTests.ProjectChronosTestsCharacter|GetbIsFacingLadder (Variables|Default|GetPlayer))
        (Variables|/Script/ProjectChronosTests.ProjectChronosTestsCharacter|SetbCanClimbLadder (Variables|Default|GetPlayer) true)
        (Pawn|Components|CharacterMovement|SetMovementMode (Variables|/Script/Engine.Character|GetCharacterMovement (Variables|Default|GetPlayer)) "MOVE_Flying" 0)
        (Variables|/Script/Engine.MovementComponent|SetVelocity (Variables|/Script/Engine.Character|GetCharacterMovement (Variables|Default|GetPlayer)) "0, 0, 0")
        (bind _alpha (Timeline|lerpPlayer PlayFromStart)
          (:Update
            (Transformation|SetWorldLocation _capsulecomponent (Math|Vector|Lerp(Vector) (Math|Vector|MakeVector (.x _returnvalue_3) (.y _returnvalue_3) (.z _returnvalue_3)) (Math|Vector|MakeVector (.x _returnvalue) (.y _returnvalue) (.z _returnvalue_3)) _alpha) false false)
            (Transformation|SetWorldRotation _capsulecomponent (Math|Rotator|FindLookatRotation (Math|Vector|MakeVector (.x _returnvalue_4) (.y _returnvalue_4) (.z _returnvalue_4)) (Math|Vector|MakeVector (.x _returnvalue_2) (.y _returnvalue_2) (.z _returnvalue_4))) false false)))))))

(event EventBeginPlay
  (bind _arrow (Variables|Default|GetArrow))
  (bind _returnvalue (Transformation|GetWorldLocation _arrow))
  (bind (_x _y _z) (Math|Vector|BreakVector _returnvalue))
  (Variables|Default|SetPlayer (.AsFirst%20Person%20Character (Utilities|Casting|CastToFirstPersonCharacter (Game|GetPlayerCharacter 0))))
  (bind _returnvalue_2 (Collision|LineTraceByChannel _returnvalue (Math|Vector|MakeVector _x _y (- _z 1e+02)) "TraceTypeQuery1" false 0 "ForDuration" true "(R=1.000000,G=0.000000,B=0.000000,A=1.000000)" "(R=0.000000,G=1.000000,B=0.000000,A=1.000000)" 0.01))
  (if (not _returnvalue_2)
    (Game|SpawnActorfromClass "BP_Ladder_C" (Math|Transform|MakeTransform (Transformation|GetWorldLocation (Variables|Default|GetArrow)) (.rotation (Transformation|GetWorldTransform (Variables|Default|GetLadder))) "1,1,1") "Undefined" 0 0)
    (Components|DestroyComponent (Variables|Default|GetLadderBox))))

(fn ConstructionScript
  (Utilities|Array|Add (Variables|/Script/Engine.ActorComponent|GetComponentTags (Variables|Default|GetLadder)) "Ladder"))