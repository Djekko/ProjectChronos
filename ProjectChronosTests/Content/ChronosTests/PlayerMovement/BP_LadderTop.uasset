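; Ladder-top actor that moves the first-person player on and off a climbable ladder, spawning a BP_Ladder at its arrow on BeginPlay.
; Overlapping either PlayerWalkAgain or Backup toggles on the player's CanClimbLadder flag, without checking the overlapping actor.
; Mounting sets Flying and zeroes velocity, while dismounting restores Walking.
; Timelines lerp the capsule horizontally to Arrow1 or the actor root, keeping its height, then flip the flag.
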(event OnComponentBeginOverlap(PlayerWalkAgain)
  (params (OverlappedComponent :type Primitive%20Component%20Object%20Reference) (OtherActor :type Actor%20Object%20Reference) (OtherComp :type Primitive%20Component%20Object%20Reference) (OtherBodyIndex :type Integer) (bFromSweep :type Boolean) (SweepResult :type Hit%20Result%20Structure%20%28by%20ref%29))
  (bind _defaultsceneroot (Variables|Default|GetDefaultSceneRoot))
  (bind _player (Variables|Default|GetPlayer))
  (bind _arrow1 (Variables|Default|GetArrow1))
  (bind _player_2 (Variables|Default|GetPlayer))
  (bind _returnvalue (Transformation|GetWorldLocation _arrow1))
  (bind _returnvalue_2 (Transformation|GetWorldLocation _defaultsceneroot))
  (bind _capsulecomponent (Variables|/Script/Engine.Character|GetCapsuleComponent _player))
  (bind _capsulecomponent_2 (Variables|/Script/Engine.Character|GetCapsuleComponent _player_2))
  (bind _returnvalue_3 (Transformation|GetWorldLocation _capsulecomponent_2))
  (bind _returnvalue_4 (Transformation|GetWorldLocation _capsulecomponent))
  (if (Variables|/Script/ProjectChronosTests.ProjectChronosTestsCharacter|GetbCanClimbLadder (Variables|Default|GetPlayer))
    (Pawn|Components|CharacterMovement|SetMovementMode (Variables|/Script/Engine.Character|GetCharacterMovement (Variables|Default|GetPlayer)) "MOVE_Walking" 0)
    (bind _alpha (Timeline|PlayerOffLadder PlayFromStart)
      (:Update
        (Transformation|SetWorldLocation (Variables|/Script/Engine.Character|GetCapsuleComponent (Variables|Default|GetPlayer)) (Math|Vector|Lerp(Vector) (Math|Vector|MakeVector (.x _returnvalue_4) (.y _returnvalue_4) (.z _returnvalue_4)) (Math|Vector|MakeVector (.x _returnvalue_2) (.y _returnvalue_2) (.z _returnvalue_4)) _alpha) false false))
      (:Finished
        (Variables|/Script/ProjectChronosTests.ProjectChronosTestsCharacter|SetbCanClimbLadder (Variables|Default|GetPlayer) false)))
    (else
      (Pawn|Components|CharacterMovement|SetMovementMode (Variables|/Script/Engine.Character|GetCharacterMovement (Variables|Default|GetPlayer)) "MOVE_Flying" 0)
      (Variables|/Script/Engine.MovementComponent|SetVelocity (Variables|/Script/Engine.Character|GetCharacterMovement (Variables|Default|GetPlayer)) "0, 0, 0")
      (bind _alpha_2 (Timeline|Timeline_0 PlayFromStart)
        (:Update
          (Transformation|SetWorldLocation (Variables|/Script/Engine.Character|GetCapsuleComponent (Variables|Default|GetPlayer)) (Math|Vector|Lerp(Vector) (Math|Vector|MakeVector (.x _returnvalue_3) (.y _returnvalue_3) (.z _returnvalue_3)) (Math|Vector|MakeVector (.x _returnvalue) (.y _returnvalue) (.z _returnvalue_3)) _alpha_2) false false))
        (:Finished
          (Variables|/Script/ProjectChronosTests.ProjectChronosTestsCharacter|SetbCanClimbLadder (Variables|Default|GetPlayer) true))))))

(event OnComponentBeginOverlap(Backup)
  (params (OverlappedComponent :type Primitive%20Component%20Object%20Reference) (OtherActor :type Actor%20Object%20Reference) (OtherComp :type Primitive%20Component%20Object%20Reference) (OtherBodyIndex :type Integer) (bFromSweep :type Boolean) (SweepResult :type Hit%20Result%20Structure%20%28by%20ref%29))
  (bind _defaultsceneroot (Variables|Default|GetDefaultSceneRoot))
  (bind _player (Variables|Default|GetPlayer))
  (bind _arrow1 (Variables|Default|GetArrow1))
  (bind _player_2 (Variables|Default|GetPlayer))
  (bind _returnvalue (Transformation|GetWorldLocation _arrow1))
  (bind _returnvalue_2 (Transformation|GetWorldLocation _defaultsceneroot))
  (bind _capsulecomponent (Variables|/Script/Engine.Character|GetCapsuleComponent _player))
  (bind _capsulecomponent_2 (Variables|/Script/Engine.Character|GetCapsuleComponent _player_2))
  (bind _returnvalue_3 (Transformation|GetWorldLocation _capsulecomponent_2))
  (bind _returnvalue_4 (Transformation|GetWorldLocation _capsulecomponent))
  (if (Variables|/Script/ProjectChronosTests.ProjectChronosTestsCharacter|GetbCanClimbLadder (Variables|Default|GetPlayer))
    (Pawn|Components|CharacterMovement|SetMovementMode (Variables|/Script/Engine.Character|GetCharacterMovement (Variables|Default|GetPlayer)) "MOVE_Walking" 0)
    (bind _alpha (Timeline|PlayerOffLadder PlayFromStart)
      (:Update
        (Transformation|SetWorldLocation (Variables|/Script/Engine.Character|GetCapsuleComponent (Variables|Default|GetPlayer)) (Math|Vector|Lerp(Vector) (Math|Vector|MakeVector (.x _returnvalue_4) (.y _returnvalue_4) (.z _returnvalue_4)) (Math|Vector|MakeVector (.x _returnvalue_2) (.y _returnvalue_2) (.z _returnvalue_4)) _alpha) false false))
      (:Finished
        (Variables|/Script/ProjectChronosTests.ProjectChronosTestsCharacter|SetbCanClimbLadder (Variables|Default|GetPlayer) false)))
    (else
      (Pawn|Components|CharacterMovement|SetMovementMode (Variables|/Script/Engine.Character|GetCharacterMovement (Variables|Default|GetPlayer)) "MOVE_Flying" 0)
      (Variables|/Script/Engine.MovementComponent|SetVelocity (Variables|/Script/Engine.Character|GetCharacterMovement (Variables|Default|GetPlayer)) "0, 0, 0")
      (bind _alpha_2 (Timeline|Timeline_0 PlayFromStart)
        (:Update
          (Transformation|SetWorldLocation (Variables|/Script/Engine.Character|GetCapsuleComponent (Variables|Default|GetPlayer)) (Math|Vector|Lerp(Vector) (Math|Vector|MakeVector (.x _returnvalue_3) (.y _returnvalue_3) (.z _returnvalue_3)) (Math|Vector|MakeVector (.x _returnvalue) (.y _returnvalue) (.z _returnvalue_3)) _alpha_2) false false))
        (:Finished
          (Variables|/Script/ProjectChronosTests.ProjectChronosTestsCharacter|SetbCanClimbLadder (Variables|Default|GetPlayer) true))))))

(event EventBeginPlay
  (Variables|Default|SetPlayer (.AsFirst%20Person%20Character (Utilities|Casting|CastToFirstPersonCharacter (Game|GetPlayerCharacter 0))))
  (Game|SpawnActorfromClass "/Game/ChronosTests/PlayerMovement/BP_Ladder.BP_Ladder_C" (Math|Transform|MakeTransform (Transformation|GetWorldLocation (Variables|Default|GetArrow)) (.rotation (Transformation|GetWorldTransform (Variables|Default|GetCube))) "1,1,1") "Undefined" 0 0))

(fn ConstructionScript)