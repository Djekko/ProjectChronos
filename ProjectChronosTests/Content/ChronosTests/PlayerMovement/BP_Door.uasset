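; BP_Door is an interactive door that swings open and closed when the first-person player triggers it.
; It binds MoveDoor to a player dispatcher and responds only when it is the player's line trace hit.
; A dot product against the door's forward vector sets swing direction from the player's side.
; A FlipFlop plays or reverses the rotation timeline, and construction tags it "door" and "SingularityExempt".
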(event Custom|MoveDoor
  (bind _self self)
  (bind _doorrotation (Variables|Default|GetDoorRotation))
  (if (== (Variables|/Script/ProjectChronosTests.ProjectChronosTestsCharacter|GetLineTraceActorHit (Variables|Default|GetPlayer)) self)
    (if (Variables|Default|GetbIsDoorOpenBP)
      _
      (elif (>= (Math|Vector|DotProduct (Class|KismetMathLibrary|GetDirectionVector (Transformation|GetActorLocation _self) (Transformation|GetActorLocation (Variables|Default|GetPlayer))) (Transformation|GetActorForwardVector _self)) 0.0)
        (Variables|Default|SetForwards/Backwards -1.0)
        (else
          (Variables|Default|SetForwards/Backwards 1.0))))
    (Utilities|FlowControl|FlipFlop
      (:A
        (Variables|Default|SetbIsDoorOpenBP true)
        (bind _doorrotation_2 (Timeline|OpenDoor Play)
          (:Update
            (Transformation|SetWorldRotation (Variables|Default|GetSM_Door) (Math|Rotator|MakeRotator (.x (+ (* _doorrotation_2 (Variables|Default|GetForwards/Backwards)) (Math|Vector|MakeVector (.roll _doorrotation) (.pitch _doorrotation) (.yaw _doorrotation)))) (.y (+ (* _doorrotation_2 (Variables|Default|GetForwards/Backwards)) (Math|Vector|MakeVector (.roll _doorrotation) (.pitch _doorrotation) (.yaw _doorrotation)))) (.z (+ (* _doorrotation_2 (Variables|Default|GetForwards/Backwards)) (Math|Vector|MakeVector (.roll _doorrotation) (.pitch _doorrotation) (.yaw _doorrotation))))) false false))))
      (:B
        (Variables|Default|SetbIsDoorOpenBP false)
        (Timeline|OpenDoor Reverse)))))

(event EventBeginPlay
  (Variables|Default|SetPlayer (.AsFirst%20Person%20Character (Utilities|Casting|CastToFirstPersonCharacter (Game|GetPlayerCharacter 0))))
  (Variables|Default|SetDoorRotation (Transformation|GetWorldRotation (Variables|Default|GetSM_Door)))
  (EventDispatchers|BindEventtoDispatchtoDoor (Variables|Default|GetPlayer) (delegate Custom|MoveDoor)))

(fn ConstructionScript
  (bind _self self)
  (bind _tags (Variables|Actor|GetTags _self))
  (Utilities|Array|Add _tags "door")
  (Utilities|Array|Add _tags "SingularityExempt"))